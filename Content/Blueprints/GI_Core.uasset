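; GI_Core is a game instance that manages the multiplayer session lifecycle and the level changes tied to it.
; CreateSession makes an advanced session for the first player controller with LAN and presence-join options, then opens the debug level on success.
; Returning to the menu, shutdown, network errors and travel errors all destroy the session, opening the main menu only if that succeeds.
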(event Custom|CreateSession
  (params (bUseLAN :type Boolean) (bAllowJoinViaPresence :type Boolean))
  (|AdvancedSession 0 (Game|GetPlayerController 0) 100 0 bUseLAN true false true bAllowJoinViaPresence false false false true false true
    (:OnSuccess
      (Game|OpenLevel(byName) "Lvl_Debug" true "?listen"))))

(event Custom|BackToMainMenu
  (|DestroySession (Game|GetPlayerController 0)
    (:OnSuccess
      (Game|OpenLevel(byName) "Lvl_MainMenu"))))

(event EventShutdown
  (|DestroySession (Game|GetPlayerController 0)
    (:OnSuccess
      (Game|OpenLevel(byName) "Lvl_MainMenu"))))

(event EventHandleNetworkError
  (params (FailureType :type ENetworkFailure%20Enum :default "NetDriverAlreadyExists") (bIsServer :type Boolean))
  (|DestroySession (Game|GetPlayerController 0)
    (:OnSuccess
      (Game|OpenLevel(byName) "Lvl_MainMenu"))))

(event EventHandleTravelError
  (params (FailureType :type ETravelFailure%20Enum :default "NoLevel"))
  (|DestroySession (Game|GetPlayerController 0)
    (:OnSuccess
      (Game|OpenLevel(byName) "Lvl_MainMenu"))))